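; BP_WeaponBase is a hitscan gun with limited ammo, a fire-rate cooldown counted in Tick and a delayed full reload.
; Shooting spends a bullet, plays sound and muzzle particles at the Arrow, then traces from the camera along the Arrow's forward vector, ignoring the shooter and weapon.
; Hits spawn an impact emitter and call Damaged on BP_NBRBasePawn targets, with damage falling linearly by distance down to MinDamage.
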(event Custom|Reload
  ;[1 1 1] Reload
  (Utilities|FlowControl|Delay 2.0)
  (Variables|Default|SetconBulletCount (Variables|Default|GetmaxBulletCount)))

(event Custom|Shooting
  (params (Camera :type Spring%20Arm%20Component%20Object%20Reference) (Person :type Capsule%20Component%20Object%20Reference))
  (bind _returnvalue (Transformation|GetWorldLocation Camera))
  (bind _mindamage (Variables|Default|GetMinDamage))
  ;[1 1 1] 사격 가능 유무 확인
  (if (Variables|Default|GetcanShooting)
    ;[1 1 1] 남은 총알 확인
    (if (> (Variables|Default|GetconBulletCount) 0)
      ;[1 1 1] 총알 수 감산, 다음 사격 딜레이 계산
      (Variables|Default|SetconDelayPerShooting 0.0)
      (Variables|Default|SetcanShooting false)
      (Variables|Default|SetconBulletCount (- (Variables|Default|GetconBulletCount) 1))
      ;[1 1 1] 사운드 재생
      (Audio|PlaySoundatLocation "/Game/MilitaryWeapDark/Sound/Rifle/Wavs/RifleB_Fire_End_ST01.RifleB_Fire_End_ST01" (Transformation|GetWorldLocation (Variables|Default|GetArrow)) "0, 0, 0" 2.0 1.0 0.0 0 0 0)
      ;[1 1 1] 총구에 불빛 추가
      (bind _returnvalue_2 (AddComponent|AddParticleSystemComponent false))
      (Transformation|SetWorldTransform _returnvalue_2 (Transformation|GetWorldTransform (Variables|Default|GetArrow)) false false)
      (bind (_outhit _returnvalue_3) (Collision|LineTraceForObjects _returnvalue (+ _returnvalue (* (Math|Vector|GetForwardVector (Variables|Default|GetArrow)) 1e+04)) (Utilities|Array|MakeArray "ObjectTypeQuery3" "ObjectTypeQuery1" "ObjectTypeQuery2" "ObjectTypeQuery4" "ObjectTypeQuery5" "ObjectTypeQuery6") true (Utilities|Array|MakeArray (Components|GetOwner Person) self) "None"))
      ;[1 1 1] 총 피격 위치에 VFX 생성
      (if _returnvalue_3
        (Effects|SpawnEmitteratLocation "/Game/MilitaryWeapDark/FX/P_SniperRifle_MuzzleFlash_01.P_SniperRifle_MuzzleFlash_01" (+ (.ImpactPoint (Collision|BreakHitResult _outhit)) (* (.ImpactNormal (Collision|BreakHitResult _outhit)) 2e+01)) "0, 0, 0" "5.000000,5.000000,5.000000")
        ;[1 1 1] \거리에 따른 데미지 감소를 포함한 사람 피격 데미지 처리
        (if (< (- (Variables|Default|GetDamage) (/ (.Distance (Collision|BreakHitResult _outhit)) 1e+03)) _mindamage)
          (bind _asbp_nbrbase_pawn (Utilities|Casting|CastToBP_NBRBasePawn (.HitActor (Collision|BreakHitResult _outhit))))
          (Default|Damaged _asbp_nbrbase_pawn _mindamage)
          (else
            (bind _asbp_nbrbase_pawn_2 (Utilities|Casting|CastToBP_NBRBasePawn (.HitActor (Collision|BreakHitResult _outhit))))
            (Default|Damaged _asbp_nbrbase_pawn_2 (- (Variables|Default|GetDamage) (/ (.Distance (Collision|BreakHitResult _outhit)) 1e+03)))))))))

(event EventBeginPlay
  ;[1 1 1] Begin Game
  (Variables|Default|SetconDelayPerShooting (Variables|Default|GetmaxDelayPerShooting))
  (Variables|Default|SetconBulletCount (Variables|Default|GetmaxBulletCount))
  (Variables|Default|SetcanShooting true))

(event EventTick
  (params (DeltaSeconds :type Float%20%28single-precision%29))
  ;[1 1 1] Shooting Delay Checking
  (if (not (Variables|Default|GetcanShooting))
    (bind _output_get (Variables|Default|SetconDelayPerShooting (+ DeltaSeconds (Variables|Default|GetconDelayPerShooting))))
    (if (>= _output_get (Variables|Default|GetmaxDelayPerShooting))
      (Variables|Default|SetcanShooting true))))

(fn ConstructionScript)