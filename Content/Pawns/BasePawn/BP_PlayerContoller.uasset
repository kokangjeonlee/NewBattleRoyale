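; Player controller for a shrinking-zone style game that handles character selection, HUD, world map and out-of-zone damage.
; SetCharacter replaces the first player's pawn with a possessed Murdock pawn at the same location and swaps in the Murdock HUD, while StartGame adds the base HUD.
; The Worldmap input toggles a cached map widget.
; Tick damages the pawn every second outside the GameState's circle, measured in 2D, and GetPawnPosition returns position and map size.
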(event Custom|StartGame
  (bind _self self)
  (bind _returnvalue (UserInterface|CreateWidget "/Game/UI/InGameHUD/HUD.HUD_C" _self _self))
  (UserInterface|Viewport|AddtoViewport _returnvalue 0))

(event Custom|SetCharacter
  (bind _returnvalue (Game|GetPlayerController 0))
  (bind _returnvalue_2 (Pawn|GetControlledPawn _returnvalue))
  (bind _output_get (Variables|Default|SetLoaction (Transformation|GetActorLocation _returnvalue_2)))
  (Actor|DestroyActor _returnvalue_2)
  (bind _returnvalue_3 (Game|SpawnActorfromClass "/Game/Pawns/BP_Pawns/BP_MurdockPawn.BP_MurdockPawn_C" (Math|Conversions|ToTransform(Vector) _output_get) "Undefined" _returnvalue 0))
  (Pawn|Possess _returnvalue _returnvalue_3)
  (Viewport|RemoveAllWidgets)
  (bind _returnvalue_4 (UserInterface|CreateWidget "/Game/Pawns/BP_Pawns/HUD_Murdock.HUD_Murdock_C" 0 0))
  (UserInterface|Viewport|AddtoViewport _returnvalue_4 0))

(event EventTick
  (params (DeltaSeconds :type Float%20%28single-precision%29))
  (bind _returnvalue (Pawn|GetControlledPawn))
  (bind _returnvalue_2 (Transformation|GetActorLocation _returnvalue))
  (bind (_x _y) (Math|Vector|BreakVector _returnvalue_2))
  (bind _output_get (Variables|Default|SetElectricDamageTime (+ DeltaSeconds (Variables|Default|GetElectricDamageTime))))
  (if (> _output_get 1.0)
    (Variables|Default|SetElectricDamageTime 0.0)
    (bind _asbp_game_state_base (Utilities|Casting|CastToBP_GameStateBase (Game|GetGameState)))
    (if (>= (Math|Vector|VectorLength (- (Math|Vector|MakeVector _x _y 0.0) (Math|Vector|MakeVector (.X (Math|Vector|BreakVector (Variables|/Game/GameState/BP_GameStateBase.BP_GameStateBase_C|GetCurrentCirclePosition _asbp_game_state_base))) (.Y (Math|Vector|BreakVector (Variables|/Game/GameState/BP_GameStateBase.BP_GameStateBase_C|GetCurrentCirclePosition _asbp_game_state_base))) 0.0))) (* (Variables|/Game/GameState/BP_GameStateBase.BP_GameStateBase_C|GetCurrentCircleRadius _asbp_game_state_base) 1e+01))
      (bind _asbp_nbrbase_pawn (Utilities|Casting|CastToBP_NBRBasePawn _returnvalue))
      (Default|Damaged _asbp_nbrbase_pawn 1e+01))))

(event Input|ActionEvents|InputActionWorldmap
  (params (Key :type Key%20Structure))
  (bind _self self)
  (:Pressed
    (Utilities|FlowControl|FlipFlop
      (:A
        (Utilities|IsValid (Variables|Default|GetWidgetBP_Worldmap)
          (:Is%20Valid
            (UserInterface|Viewport|AddtoViewport (Variables|Default|GetWidgetBP_Worldmap) 0))
          (:Is%20Not%20Valid
            (bind _returnvalue (UserInterface|CreateWidget "/Game/Worldmap/WidgetBP_Worldmap.WidgetBP_Worldmap_C" _self _self))
            (bind _output_get (Variables|Default|SetWidgetBP_Worldmap _returnvalue))
            (UserInterface|Viewport|AddtoViewport _output_get 0))))
      (:B
        (Utilities|IsValid (Variables|Default|GetWidgetBP_Worldmap)
          (:Is%20Valid
            (Widget|RemovefromParent (Variables|Default|GetWidgetBP_Worldmap))))))))

(fn ConstructionScript)

(fn GetPawnPosition
  (bind _returnvalue (Pawn|GetControlledPawn))
  (Utilities|IsValid _returnvalue
    (:Is%20Valid
      (return (Transformation|GetActorLocation _returnvalue) (Variables|Default|GetMapSize)))
    (:Is%20Not%20Valid
      (return "100000000376832.000000,100000000376832.000000,0.000000" (Variables|Default|GetMapSize)))))