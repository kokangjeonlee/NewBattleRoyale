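; BP_GameMode is a game mode that switches the default pawn class to match a selected character.
; ChangeDefaultPawn destroys player controller 0, then maps Sian, Murdock, Trapper or Wraith to its pawn Blueprint, falling back to BP_NBRBasePawn.
; It only sets the class and prints debug strings, with no spawn or possession in this graph.
; ChangeDefaultWeapon, BeginPlay, Tick and the construction script are empty.
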(event EventBeginPlay)

(event EventTick
  (params (DeltaSeconds :type Float%20%28single-precision%29)))

(fn ConstructionScript)

(fn ChangeDefaultPawn
  (params (character :type String))
  (bind _sian (LocalVariables|GetSian))
  (Development|PrintString "Im in change default pawn")
  (Actor|DestroyActor (Game|GetPlayerController 0))
  (if (Utilities|Enum|Equal(Enum) character _sian)
    (Variables|Default|SetDefaultPawnClass "/Game/Pawns/BP_Pawns/BP_SianPawn.BP_SianPawn_C")
    (Development|PrintString _sian)
    (elif (Utilities|Enum|Equal(Enum) character (LocalVariables|GetMurdock))
      (Variables|Default|SetDefaultPawnClass "/Game/Pawns/BP_Pawns/BP_MurdockPawn.BP_MurdockPawn_C")
      (elif (Utilities|Enum|Equal(Enum) character (LocalVariables|GetTrapper))
        (Variables|Default|SetDefaultPawnClass "/Game/Pawns/BP_Pawns/BP_TrapperPawn.BP_TrapperPawn_C")
        (elif (Utilities|Enum|Equal(Enum) character (LocalVariables|GetWraith))
          (Variables|Default|SetDefaultPawnClass "/Game/Pawns/BP_Pawns/BP_WraithPawn.BP_WraithPawn_C")
          (else
            (Variables|Default|SetDefaultPawnClass "/Game/Pawns/BP_Pawns/BP_NBRBasePawn.BP_NBRBasePawn_C")))))))

(fn ChangeDefaultWeapon)